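; Example actor that renders Niagara GPU particles as Nanite instanced static meshes through particle data export.
; On BeginPlay it registers as the Niagara callback handler and sets the GPU readback limit.
; Each callback converts particle data into per-mesh transform arrays in C++, then creates or refills one ISM component per mesh index.
; A DoOnce reset next tick drops duplicate same-frame readbacks, and Tick drives a throttled FPS display.
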(event `self.ReceiveBeginPlay`
  ;[1 1 1] Tells Niagara to Call-Back to Self(this actor) and execute the export of Particle Array Data via "Event Recieve Particle Data"
  (`NiagaraComponent.SetVariableObject` (`self.AggM_Example_exportNiagaraSystem`) "CallBackHandler" self)
  (`KismetSystemLibrary.ExecuteConsoleCommand` "fx.Niagara.NDIExport.GPUMaxReadbackCount 110000" null))

(event `self.ReceiveTick`
  (params (DeltaSeconds :type "Float (single-precision)"))
  ;[1 1 1] Low Refresh FPS
  (`KismetSystemLibrary.Delay` 0.1)
  (`TextRenderComponent.K2_SetText` (`self.FPS_Display`) (`KismetTextLibrary.Conv_StringToText` (`KismetStringLibrary.Concat_StrStr` (`KismetStringLibrary.Conv_IntToString` (`KismetMathLibrary.Round` (/ 1.0 DeltaSeconds))) " FPS"))))

(event `self.ReceiveParticleData`
  (params (Data :type "Array of BasicParticleData Structure (by ref)") (NiagaraSystem :type "NiagaraSystem Object Reference") (SimulationPositionOffset :type "Vector Structure (by ref)"))
  (bind _spawnedismarrays (`self.SpawnedISMArrays`))
  ;[1 1 1] Call-Back Event from Niagara with Particle Data in one Array
  ;[1 1 1] GPU will report back twice a frame sometimes...
  (`/Engine/EditorBlueprintResources/StandardMacros.DoOnce` false :!label _label
    (:`Completed`
      ;[1 1 1] Loop to Convert Particle Packed Data into Transform Arrays by Mesh Index in C++
      (bind _returnvalue (`AggM_NiagaraNaniteConvertBPLibrary.GPUExportCPP` Data))
      ;[1 1 1] Nanite Rendering Update Each Call
      (for (_array_element _array_index) _returnvalue
        (if (`KismetArrayLibrary.Array_IsValidIndex` _spawnedismarrays _array_index)
          (bind _output (`|GetArrayItem` _spawnedismarrays _array_index))
          (`InstancedStaticMeshComponent.ClearInstances` _output)
          (bind _positions (break `NiagaraExportData` _array_element))
          (`InstancedStaticMeshComponent.AddInstances` _output _positions false true)
          (else
            (bind _returnvalue_2 (`AddComponent|NODE_AddInstancedStaticMeshComponent-0` :`RelativeTransform` (`KismetMathLibrary.MakeTransform` (0.0 0.0 0.0) (struct) (5.0 5.0 5.0))))
            (`KismetArrayLibrary.Array_Add` _spawnedismarrays _returnvalue_2)
            (`PrimitiveComponent.SetAffectDistanceFieldLighting` _returnvalue_2 false)
            (`StaticMeshComponent.SetStaticMesh` _returnvalue_2 (`|GetArrayItem` (`self.MatchingMeshIndexArray`) _array_index))
            (`PrimitiveComponent.SetMaterial` _returnvalue_2 0 "/AggM_NiagaraNaniteConvert/Materials/NaniteISMMaterial.NaniteISMMaterial")
            (`PrimitiveComponent.SetCollisionEnabled` _returnvalue_2 "NoCollision")
            (`SceneComponent.SetMobility` _returnvalue_2 "Movable")
            (`PrimitiveComponent.SetCollisionResponseToAllChannels` _returnvalue_2 "ECR_Ignore")
            (set `PrimitiveComponent.bGenerateOverlapEvents` false _returnvalue_2)
            (set `PrimitiveComponent.CanCharacterStepUpOn` "ECB_No" _returnvalue_2)
            (`InstancedStaticMeshComponent.AddInstances` _returnvalue_2 _positions false true))))
      (`KismetSystemLibrary.DelayUntilNextTick`)
      (goto _label :!via `Reset`))))

(fn `UserConstructionScript`)